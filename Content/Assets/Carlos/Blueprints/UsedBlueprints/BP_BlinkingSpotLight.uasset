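; Blinking light actor that sets a color on its PointLight component and optionally flickers it at random intervals.
; BeginPlay applies the color and holds the light at maximum intensity when flickering is off.
; Tick runs Flicker, which waits a random delay between its bounds, then sets intensity to a random blend of the minimum and maximum.
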(event `self.ReceiveBeginPlay`
  (`LightComponent.SetLightColor` (`self.PointLight`) (`KismetMathLibrary.Conv_ColorToLinearColor` (`self.In SRGB`)) true)
  (if (not (`self.lightFlickers?`))
    (`LightComponent.SetIntensity` (`self.PointLight`) (`self.max intensity`))))

(event `self.ReceiveTick`
  (params (DeltaSeconds :type "Float (single-precision)"))
  (`self.Flicker` (`self.lightFlickers?`) (`self.min delay`) (`self.max delay`) (`self.min intensity`) (`self.max intensity`) (`self.PointLight`)))

(fn `UserConstructionScript`)