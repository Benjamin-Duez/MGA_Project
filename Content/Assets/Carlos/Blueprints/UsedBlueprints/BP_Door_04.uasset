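; BP_Door_04 is a swinging door that opens and closes automatically for BP_TopDownCharacter when CanOpen is set.
; Box overlap begin plays DoorTimeline and overlap end reverses it, both gated by CanOpen and a character cast.
; The timeline scales the AngleOuverurePorte opening angle to set PivotAxis relative yaw, with InvertAnimation flipping the swing direction.
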(event `self.Box.OnComponentBeginOverlap`
  (params (OverlappedComponent :type "PrimitiveComponent Object Reference") (OtherActor :type "Actor Object Reference") (OtherComp :type "PrimitiveComponent Object Reference") (OtherBodyIndex :type Integer) (bFromSweep :type Boolean) (SweepResult :type "HitResult Structure (by ref)"))
  (bind _angleouverureporte (`self.AngleOuverurePorte`))
  (if (`self.canOpen`)
    (castclass `Actor` "/Game/TopDown/Blueprints/BP_TopDownCharacter.BP_TopDownCharacter_C")
    (bind (_direction _doortimeline) (`Timeline|DoorTimeline` :!label _label)
      (:`Update`
        (`SceneComponent.K2_SetRelativeRotation` (`self.PivotAxis`) (`KismetMathLibrary.MakeRotator` 0.0 0.0 (* _doortimeline (select `bool` (`self.InvertAnimation`) :`false` _angleouverureporte :`true` (* _angleouverureporte -1.0)))) false false)))))

(event `self.Box.OnComponentEndOverlap`
  (params (OverlappedComponent :type "PrimitiveComponent Object Reference") (OtherActor :type "Actor Object Reference") (OtherComp :type "PrimitiveComponent Object Reference") (OtherBodyIndex :type Integer))
  (if (`self.canOpen`)
    (castclass `Actor` "/Game/TopDown/Blueprints/BP_TopDownCharacter.BP_TopDownCharacter_C")
    (goto _label :!via `Reverse`)))

(fn `UserConstructionScript`)