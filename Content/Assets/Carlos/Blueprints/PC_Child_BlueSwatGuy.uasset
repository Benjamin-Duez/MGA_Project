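; Child character Blueprint for the blue SWAT guy, with a rifle mesh and state getters.
; SwitchWeapon sets the Rifle component's skeletal mesh to the Val model or clears it, and construction defers to the parent.
; Getters expose the muzzle socket transform, movement velocity and location, faction, range flag, montage state and health, while the display name returns empty.
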(event `self.ReceiveBeginPlay`)

(event `/Game/Assets/Carlos/Blueprints/BPI_PlayerCharacterStatus.SwitchWeapon`
  (params (NewParam :type "/Game/Characters/WeaponsSelectionEnum Enum" :default "NewEnumerator3"))
  (bind _rifle (`self.Rifle`))
  (switch `/Game/Characters/WeaponsSelectionEnum` NewParam
    (:`NewEnumerator3`
      (`SkinnedMeshComponent.SetSkinnedAssetAndUpdate` _rifle null false))
    (:`NewEnumerator1`
      (`SkinnedMeshComponent.SetSkinnedAssetAndUpdate` _rifle "/Game/FPS_Weapon_Bundle/Weapons/Meshes/KA_Val/SK_KA_Val_Y.SK_KA_Val_Y" false))))

(fn `GetCanonSocket`
  (returns (RifleSocketTrans :type "Transform Structure"))
  (return (`SceneComponent.GetSocketTransform` (`self.Rifle`) "CanonSocket" "RTS_World")))

(fn `GetCharacterLocation`
  (returns (Location :type "Vector Structure"))
  (return (`CharacterMovementComponent.GetLastUpdateLocation` (`self.CharacterMovement`))))

(fn `GetCharacterVelocity`
  (returns (Velocity :type "Vector Structure") (Lenght :type "Float (double-precision)"))
  (bind _velocity (`MovementComponent.Velocity` (`self.CharacterMovement`)))
  (return _velocity (`KismetMathLibrary.VSize` _velocity)))

(fn `GetCurrentHealth`
  (returns (currentHealth :type "Float (double-precision)"))
  (return (`self.CurrentHealth`)))

(fn `GetDisplayName`
  (returns (DisplayName :type Text))
  (return ""))

(fn `GetFaction`
  (returns (Faction :type "/Game/Characters/CharacterFaction Enum"))
  (return (`self.Faction`)))

(fn `GetIsInRange`
  (returns (isInRange :type Boolean))
  (return (`self.isInRange`)))

(fn `GetMaxHealth`
  (returns (maxHealth :type "Float (double-precision)"))
  (return (`self.MaxHealth`)))

(fn `GetMontagePlaying`
  (returns (isMontagePlaying :type Boolean))
  (return (`self.isMontagePlaying`)))

(fn `UserConstructionScript`
  (`parent.UserConstructionScript`))