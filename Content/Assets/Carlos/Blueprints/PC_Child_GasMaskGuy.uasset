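; Gas mask guy character Blueprint, a child class that exposes its state through getter functions.
; The getters return velocity and speed, location, faction, display name, current and max health, range and montage flags, and the rifle's CanonSocket world transform.
; The construction script only calls the parent's, and the event graph holds only disabled placeholder events, so this child adds no event logic of its own.
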(fn `GetCanonSocket`
  (returns (RifleSocketTrans :type "Transform Structure"))
  (return (`SceneComponent.GetSocketTransform` (`self.Rifle`) "CanonSocket" "RTS_World")))

(fn `GetCharacterLocation`
  (returns (Location :type "Vector Structure"))
  (return (`self.K2_GetActorLocation` self)))

(fn `GetCharacterVelocity`
  (returns (Velocity :type "Vector Structure") (Lenght :type "Float (double-precision)"))
  (bind _velocity (`MovementComponent.Velocity` (`self.CharacterMovement`)))
  (return _velocity (`KismetMathLibrary.VSize` _velocity)))

(fn `GetCurrentHealth`
  (returns (currentHealth :type "Float (double-precision)"))
  (return (`self.CurrentHealth`)))

(fn `GetDisplayName`
  (returns (DisplayName :type Text))
  (return (`self.CharacterNameUI`)))

(fn `GetFaction`
  (returns (Faction :type "/Game/Characters/CharacterFaction Enum"))
  (return (`self.Faction`)))

(fn `GetIsInRange`
  (returns (isInRange :type Boolean))
  (return (`self.isInRange`)))

(fn `GetMaxHealth`
  (returns (maxHealth :type "Float (double-precision)"))
  (return (`self.MaxHealth`)))

(fn `GetMontagePlaying`
  (returns (isMontagePlaying :type Boolean))
  (return (`self.isMontagePlaying`)))

(fn `UserConstructionScript`
  (`parent.UserConstructionScript`))