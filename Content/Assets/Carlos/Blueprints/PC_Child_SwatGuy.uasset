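; PC_Child_SwatGuy is a child character Blueprint for a SWAT guy that adds weapon visuals and exposes character state.
; SwitchWeapon swaps the mesh on the Rifle skeletal component between none, an M9 knife and an AR4 rifle without reinitializing the pose.
; Getter functions report velocity, location, muzzle socket transform, range flag, faction, display name, montage state and health.
; Construction defers to the parent, and BeginPlay, overlap and Tick are unused.
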(event `/Game/Assets/Carlos/Blueprints/BPI_PlayerCharacterStatus.SwitchWeapon`
  (params (NewParam :type "/Game/Characters/WeaponsSelectionEnum Enum" :default "NewEnumerator0"))
  (bind _rifle (`self.Rifle`))
  (switch `/Game/Characters/WeaponsSelectionEnum` NewParam
    (:`NewEnumerator3`
      (`SkinnedMeshComponent.SetSkinnedAssetAndUpdate` _rifle null false))
    (:`NewEnumerator0`
      (`SkinnedMeshComponent.SetSkinnedAssetAndUpdate` _rifle "/Game/FPS_Weapon_Bundle/Weapons/Meshes/M9_Knife/SK_M9_Knife_Z_Up.SK_M9_Knife_Z_Up" false))
    (:`NewEnumerator1`
      (`SkinnedMeshComponent.SetSkinnedAssetAndUpdate` _rifle "/Game/FPS_Weapon_Bundle/Weapons/Meshes/AR4/SK_AR4.SK_AR4" false))))

(fn `GetCanonSocket`
  (returns (RifleSocketTrans :type "Transform Structure"))
  (return (`SceneComponent.GetSocketTransform` (`self.Rifle`) "CanonSocket" "RTS_World")))

(fn `GetCharacterLocation`
  (returns (Location :type "Vector Structure"))
  (return (`self.K2_GetActorLocation`)))

(fn `GetCharacterVelocity`
  (returns (Velocity :type "Vector Structure") (Lenght :type "Float (double-precision)"))
  (bind _velocity (`MovementComponent.Velocity` (`self.CharacterMovement`)))
  (return _velocity (`KismetMathLibrary.VSize` _velocity)))

(fn `GetCurrentHealth`
  (returns (currentHealth :type "Float (double-precision)"))
  (return (`self.CurrentHealth`)))

(fn `GetDisplayName`
  (returns (DisplayName :type Text))
  (return (`self.CharacterNameUI`)))

(fn `GetFaction`
  (returns (Faction :type "/Game/Characters/CharacterFaction Enum"))
  (return (`self.Faction`)))

(fn `GetIsInRange`
  (returns (isInRange :type Boolean))
  (return (`self.isInRange`)))

(fn `GetMaxHealth`
  (returns (maxHealth :type "Float (double-precision)"))
  (return (`self.MaxHealth`)))

(fn `GetMontagePlaying`
  (returns (isMontagePlaying :type Boolean))
  (return (`self.isMontagePlaying`)))

(fn `UserConstructionScript`
  (`parent.UserConstructionScript`))