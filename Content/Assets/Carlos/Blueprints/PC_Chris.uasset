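; Playable character Blueprint for Chris, with click-to-move, mouse-drag camera yaw, health and montage-driven active skills.
; Construction loads name, faction and health from a data table, scales the attack-range sphere and binds modular meshes to the body.
; Clicks move toward the cursor point or target pawn, while sphere overlaps track in-range faction actors.
; Possession toggles the ground marker and fills the HUD through interface messages, which also receive damage updates.
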(event `PlayShootMontage`
  ;[1 1 1] Shoot Montage
  (`self.PlayAnimMontage` (`self.MontageSkill`)))

(event `InputAxis|Look Yaw`
  (params (AxisValue :type "Float (single-precision)"))
  (bind (_locationx _locationy _returnvalue) (`PlayerController.GetMousePosition` (`GameplayStatics.GetPlayerController` 0)))
  (bind _returnvalue_2 (- (`KismetMathLibrary.MakeVector2D` _locationx _locationy) (`self.mouseLookYaw`)))
  ;[1 1 1] LookAround
  (`/Engine/EditorBlueprintResources/StandardMacros.Gate` true :!label _label
    (:`Exit`
      (`SceneComponent.K2_AddRelativeRotation` (`self.SpringArm`) (`KismetMathLibrary.MakeRotator` 0.0 0.0 (* (`KismetMathLibrary.FClamp` (* (* (`self.cameraYawSensibility`) 0.01) (`KismetMathLibrary.VSize2D` _returnvalue_2)) 0.0 2.5) (`KismetMathLibrary.BreakVector2D` (`KismetMathLibrary.Normal2D` _returnvalue_2)))) false false))))

(event `InputAction|LookAround`
  (params (Key :type "Key Structure"))
  (bind (_locationx _locationy _returnvalue) (`PlayerController.GetMousePosition` (`GameplayStatics.GetPlayerController` 0)))
  ;[1 1 1] LookAround
  (:`Pressed`
    (`|ExecutionSequence`
      (:`then_0`
        (goto _label :!via `Open`))
      (:`then_1`
        (if _returnvalue
          (`/Engine/EditorBlueprintResources/StandardMacros.DoOnce` false :!label _label_2
            (:`Completed`
              (set `self.mouseLookYaw` (`KismetMathLibrary.MakeVector2D` _locationx _locationy))))))))
  (:`Released`
    (`|ExecutionSequence`
      (:`then_0`
        (goto _label :!via `Close`))
      (:`then_1`
        (goto _label_2 :!via `Reset`)))))

(event `/Game/Assets/Carlos/Blueprints/BPI_PlayerCharacterMovement.Move2Destination`
  ;[0.02083 0.02083 0.02083] Movement
  (bind _clickedactor (`self.GetClickedActor`))
  (`/Engine/EditorBlueprintResources/StandardMacros.IsValid` _clickedactor
    (:`Is Valid`
      (bind _output_get (set `self.TargetActor` _clickedactor))
      (if (`self.isInRange`)
        (`KismetSystemLibrary.Delay` 1.0)
        (`MovementComponent.StopMovementImmediately` (`self.CharacterMovement`))
        (else
          (`self.MoveToActor` _output_get))))
    (:`Is Not Valid`
      (`self.Move To Clicked Position`))))

(event `self.ReceivePossessed`
  (params (NewController :type "Controller Object Reference"))
  ;[0.02083 0.02083 0.02083] On Posses
  (`|ExecutionSequence`
    (:`then_0`
      (`self.SetHUDCharacterData` NewController))
    (:`then_1`
      (if (`Controller.IsPlayerController` NewController)
        (`SceneComponent.SetVisibility` (`self.Ground Marker`) true false)))))

(event `self.ReceiveUnpossessed`
  (params (OldController :type "Controller Object Reference"))
  ;[0.02083 0.02083 0.02083] On Unposses
  (`SceneComponent.SetVisibility` (`self.Ground Marker`) false false))

(event `self.AttackRange.OnComponentBeginOverlap`
  (params (OverlappedComponent :type "PrimitiveComponent Object Reference") (OtherActor :type "Actor Object Reference") (OtherComp :type "PrimitiveComponent Object Reference") (OtherBodyIndex :type Integer) (bFromSweep :type Boolean) (SweepResult :type "HitResult Structure (by ref)"))
  (if (`KismetSystemLibrary.DoesImplementInterface` OtherActor "/Game/Assets/Carlos/Blueprints/BPI_Faction.BPI_Faction_C")
    (set `self.isInRange` true)
    (bind _output_get (set `self.TargetActor` OtherActor))
    (`/Engine/EditorBlueprintResources/StandardMacros.IsValid` _output_get
      (:`Is Valid`
        (`KismetSystemLibrary.PrintString` "is valid actor"))
      (:`Is Not Valid`
        (`KismetSystemLibrary.PrintString` "not valid actor")))))

(event `self.AttackRange.OnComponentEndOverlap`
  (params (OverlappedComponent :type "PrimitiveComponent Object Reference") (OtherActor :type "Actor Object Reference") (OtherComp :type "PrimitiveComponent Object Reference") (OtherBodyIndex :type Integer))
  (if (`KismetSystemLibrary.DoesImplementInterface` OtherActor "/Game/Assets/Carlos/Blueprints/BPI_Faction.BPI_Faction_C")
    (set `self.isInRange` false)
    (set `self.TargetActor` null)))

(event `self.ReceiveAnyDamage`
  (params (Damage :type "Float (single-precision)") (DamageType :type "DamageType Object Reference") (InstigatedBy :type "Controller Object Reference") (DamageCauser :type "Actor Object Reference"))
  (bind _currenthp (`self.ApplyDamageToHealth` Damage))
  (if (`self.IsPlayerControlled` self)
    (message `/Game/UI/BPI_HUD.UpdateHealthBar` (`PlayerController.GetHUD` (`GameplayStatics.GetPlayerController` 0)) _currenthp)))

(event `/Game/Assets/Carlos/Blueprints/BPI_PlayerCharacterStatus.PlayActiveSkill`
  (params (ActiveSkill :type "/Game/UI/Enum_ActiveSkill Enum" :default "NewEnumerator0") (relaunchDelay :type "Float (double-precision)"))
  (`self.PlaySkillMontage` ActiveSkill))

(fn `ApplyDamageToHealth`
  (params (damageTaken :type "Float (double-precision)"))
  (returns (currentHp :type "Float (double-precision)"))
  (bind _output_get (set `self.CurrentHealth` (`KismetMathLibrary.FClamp` (- (`self.CurrentHealth`) damageTaken) 0.0 (`self.MaxHealth`))))
  (return _output_get))

(fn `Get Destination to Move`
  (returns (Destination :type "Vector Structure"))
  (return (`.Location` (`GameplayStatics.BreakHitResult` (`PlayerController.GetHitResultUnderCursorByChannel` (`GameplayStatics.GetPlayerController` 0) "TraceTypeQuery1" true)))))

(fn `GetCanonSocket`
  (returns (RifleSocketTrans :type "Transform Structure"))
  (return (`SceneComponent.GetSocketTransform` (`self.Rifle`) "CanonSocket" "RTS_World")))

(fn `GetCharacterLocation`
  (returns (Location :type "Vector Structure"))
  (return (`CharacterMovementComponent.GetLastUpdateLocation` (`self.CharacterMovement`))))

(fn `GetCharacterVelocity`
  (returns (Velocity :type "Vector Structure") (Lenght :type "Float (double-precision)"))
  (bind _velocity (`MovementComponent.Velocity` (`self.CharacterMovement`)))
  (return _velocity (`KismetMathLibrary.VSize` _velocity)))

(fn `GetClickedActor`
  (returns (ClickedActor :type "Actor Object Reference"))
  (return (`.HitActor` (`GameplayStatics.BreakHitResult` (`PlayerController.GetHitResultUnderCursorForObjects` (`GameplayStatics.GetPlayerController` 0) (`|MakeArray` "ObjectTypeQuery3" :!type "EObjectTypeQuery Enum") true)))))

(fn `GetCurrentHealth`
  (returns (currentHealth :type "Float (double-precision)"))
  (return 0.0))

(fn `GetDisplayName`
  (returns (DisplayName :type Text))
  (return ""))

(fn `GetFaction`
  (returns (Faction :type "/Game/Characters/CharacterFaction Enum"))
  (return (`self.Faction`)))

(fn `GetIsAttacking`
  (returns (isAttacking :type Boolean))
  (return (`self.isMontagePlaying`)))

(fn `GetIsInRange`
  (returns (isInRange :type Boolean))
  (return (`self.isInRange`)))

(fn `GetMaxHealth`
  (returns (maxHealth :type "Float (double-precision)"))
  (return 0.0))

(fn `Move To Clicked Position`
  (bind _charactermovement (`self.CharacterMovement`))
  (bind _destination (`self.Get Destination to Move`))
  (bind _output_get (set `self.MoveDestination` _destination))
  (if (> (`KismetMathLibrary.VSize` (- _output_get (`self.K2_GetActorLocation`))) 150.0)
    (set `CharacterMovementComponent.MaxWalkSpeed` 600.0 _charactermovement)
    (else
      (set `CharacterMovementComponent.MaxWalkSpeed` 150.0 _charactermovement)))
  (`AIBlueprintHelperLibrary.SimpleMoveToLocation` (`self.GetController`) (`self.MoveDestination`)))

(fn `MoveToActor`
  (params (MoveToActor :type "Actor Object Reference"))
  (`AIBlueprintHelperLibrary.SimpleMoveToActor` (`GameplayStatics.GetPlayerController` 0) MoveToActor))

(fn `SetHUDCharacterData`
  (params (Controller :type "Controller Object Reference"))
  (bind _returnvalue (`PlayerController.GetHUD` (`GameplayStatics.GetPlayerController` 0)))
  (if (`Controller.IsPlayerController` Controller)
    (if (`KismetSystemLibrary.DoesImplementInterface` _returnvalue "/Game/UI/BPI_HUD.BPI_HUD_C")
      (bind _returnvalue_2 (`|GetDataTableRow` (`self.CharactersDataTable`) (`self.RowName`))
        (:`then`
          (bind (_name _faction _maxhp _charactericon _skill1_icon _skill2_icon _skill3_icon) (break `/Game/Characters/CharacterDataStructure` _returnvalue_2))
          (message `/Game/UI/BPI_HUD.SetHealthBarData` _returnvalue _name _maxhp (`self.CurrentHealth`) _charactericon)
          (message `/Game/UI/BPI_HUD.SetSkillsIcons` _returnvalue _skill1_icon _skill2_icon _skill3_icon)))
      (else
        (`KismetSystemLibrary.PrintString` "Not HUD interface found")))))

(fn `UpdateMontageStatus`
  (params (ActiveSkill :type "/Game/UI/Enum_ActiveSkill Enum" :default "NewEnumerator0") (isCompleted :type Boolean))
  (message `/Game/UI/BPI_HUD.UpdateMontageStatus` (`PlayerController.GetHUD` (`GameplayStatics.GetPlayerController` 0)) ActiveSkill isCompleted))

(fn `UserConstructionScript`
  (`|ExecutionSequence`
    (:`then_0`
      (`SphereComponent.SetSphereRadius` (`self.AttackRange`) (* (`self.attackRangeRadius`) (`SphereComponent.GetUnscaledSphereRadius` (`self.AttackRange`))) true))
    (:`then_1`
      (bind _output_get (set `self.RowName` (`KismetStringLibrary.Conv_StringToName` (`|GetEnumeratorNameAsString` (`self.CharacterSelection`)))))
      (bind _returnvalue (`|GetDataTableRow` (`self.CharactersDataTable`) _output_get)
        (:`then`
          (bind (_name _faction _maxhp) (break `/Game/Characters/CharacterDataStructure` _returnvalue))
          (set `self.CharacterNameUI` _name)
          (set `self.Faction` _faction)
          (bind _output_get_2 (set `self.MaxHealth` _maxhp))
          (set `self.CurrentHealth` _output_get_2))))
    (:`then_2`
      (`SkinnedMeshComponent.SetLeaderPoseComponent` (`self.Hair`) (`self.Body`) false)
      (`SkinnedMeshComponent.SetLeaderPoseComponent` (`self.Head`) (`self.Body`) false)
      (`SkinnedMeshComponent.SetLeaderPoseComponent` (`self.Eyes`) (`self.Body`) false)
      (`SkinnedMeshComponent.SetLeaderPoseComponent` (`self.Coat`) (`self.Body`) false))))