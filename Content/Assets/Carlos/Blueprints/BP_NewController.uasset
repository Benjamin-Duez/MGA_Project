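; Player controller for click-to-move play that switches possession among the level's PlayerCharacters and a free-view spectator camera.
; It gathers characters after a short delay on BeginPlay, then possesses by cycling or number keys; free view toggles to a camera spawned behind the character.
; Set-destination clicks message the character to move and show a Niagara cursor on flat ground free of pawns or faction actors.
; It also has a HUD update helper and unused target-point spawning.
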(event `self.ReceiveBeginPlay`
  (`|ExecutionSequence`
    (:`then_0`
      ;[0.02083 0.02083 0.02083] Find player characters by class
      (`KismetSystemLibrary.Delay` 0.2)
      (bind _outactors (`GameplayStatics.GetAllActorsOfClass` "/Game/Assets/Carlos/Blueprints/PlayerCharacter.PlayerCharacter_C"))
      (set `self.Characters` _outactors)
      (`self.Posses Character`)
      (`WidgetBlueprintLibrary.SetFocusToGameViewport`)
      (set `self.bShowMouseCursor` true))))

(event `InputAction|FreeView`
  (params (Key :type "Key Structure"))
  ;[0.02083 0.02083 0.02083] Switch Spectator/Character
  (:`Pressed`
    (if (`KismetSystemLibrary.DoesImplementInterface` (`GameplayStatics.GetPlayerPawn` 0) "/Game/Assets/Carlos/Blueprints/BPI_PlayerCharacterMovement.BPI_PlayerCharacterMovement_C")
      (bind _returnvalue (`self.SpawnSpectatorCam`))
      (`self.Possess` _returnvalue)
      (else
        (`self.Posses Character`)))))

(event `InputAction|select_character`
  (params (Key :type "Key Structure"))
  ;[0.02083 0.02083 0.02083] Character Switching
  ;;[0.02083 0.02083 0.02083] Switch Characters sequentially - Tab Key
  (:`Pressed`
    (`self.Increase Character Index`)
    (`self.Posses Character`)))

(event `InputAction|SwitchToCharacter1`
  (params (Key :type "Key Structure"))
  ;[0.02083 0.02083 0.02083] Character Switching
  ;;[0.02083 0.02083 0.02083] Character switch - Number Keys
  (:`Pressed`
    (set `self.CurrentCharacter` 0)
    (`self.Posses Character`)))

(event `InputAction|SwitchToCharacter2`
  (params (Key :type "Key Structure"))
  ;[0.02083 0.02083 0.02083] Character Switching
  ;;[0.02083 0.02083 0.02083] Character switch - Number Keys
  (:`Pressed`
    (set `self.CurrentCharacter` 1)
    (`self.Posses Character`)))

(event `self.ReceiveTick`
  (params (DeltaSeconds :type "Float (single-precision)"))
  ;[0.02083 0.02083 0.02083] Tick
)

(event `InputAction|SwitchToCharacter3`
  (params (Key :type "Key Structure"))
  ;[0.02083 0.02083 0.02083] Character Switching
  ;;[0.02083 0.02083 0.02083] Character switch - Number Keys
  (:`Pressed`
    (set `self.CurrentCharacter` 1)
    (`self.Posses Character`)))

(event `InputAction|SetDestination`
  (params (Key :type "Key Structure"))
  (bind (_hitresult _returnvalue) (`self.GetHitResultUnderCursorByChannel` "TraceTypeQuery1" false))
  (bind (_bblockinghit _binitialoverlap _time _distance _location _impactpoint _normal _impactnormal _physmat _hitactor) (`GameplayStatics.BreakHitResult` _hitresult))
  ;[0.02083 0.02083 0.02083] Spawn Niagara Destination Cursor
  (:`Pressed`
    (`/Engine/EditorBlueprintResources/StandardMacros.DoOnce` false :!label _label
      (:`Completed`
        (if _returnvalue
          (message `/Game/Assets/Carlos/Blueprints/BPI_PlayerCharacterMovement.Move2Destination` (`GameplayStatics.GetPlayerCharacter` 0))
          (if (not (`.ReturnValue` (`self.GetHitResultUnderCursorForObjects` (`|MakeArray` "ObjectTypeQuery3" :!type "EObjectTypeQuery Enum"))))
            (if (== _impactnormal (0.0 0.0 1.0) :`ErrorTolerance` 0.3)
              (if (not (`KismetSystemLibrary.DoesImplementInterface` _hitactor "/Game/Assets/Carlos/Blueprints/BPI_Faction.BPI_Faction_C"))
                (`NiagaraFunctionLibrary.SpawnSystemAtLocation` "/Game/Cursor/FX_Cursor.FX_Cursor" _location (struct) (1.0 1.0 1.0) true true "AutoRelease"))))))))
  (:`Released`
    (goto _label :!via `Reset`)))

(fn `FinTargetPoints`
  (bind _outactors (`GameplayStatics.GetAllActorsOfClass` "/Script/Engine.TargetPoint"))
  (bind _output_get (set `self.SpawnTargets` _outactors))
  (`KismetArrayLibrary.Array_Reverse` _output_get))

(fn `Get Character Last Frame Speed`
  (returns (SpeedMagnitude :type "Float (double-precision)"))
  (return (`KismetMathLibrary.VSize` (`CharacterMovementComponent.GetLastUpdateVelocity` (`Character.CharacterMovement` (`|GetArrayItem` (`self.Characters`) (`self.CurrentCharacter`)))))))

(fn `Get Destination To move`
  (returns (Destination :type "Vector Structure"))
  (return (`.Location` (`GameplayStatics.BreakHitResult` (`self.GetHitResultUnderCursorByChannel` self "TraceTypeQuery1" true)))))

(fn `GetActiveCharacter`
  (returns (NewParam :type "/Game/DataAssets/PlayerCharactersData Structure"))
  (return))

(fn `Increase Character Index`
  (bind _result (`/Engine/EditorBlueprintResources/StandardMacros.IncrementInt` (`self.CurrentCharacter`))
    (:`  `
      (set `self.CurrentCharacter` (mod _result (`KismetArrayLibrary.Array_Length` (`self.Characters`))))
      (return))))

(fn `Move To Clicked Position`
  (bind _destination (`self.Get Destination To move`))
  (set `self.MoveDestination` _destination)
  (if true
    _))

(fn `Posses Character`
  (`self.Possess` (`|GetArrayItem` (`self.Characters`) (`self.CurrentCharacter`))))

(fn `SpawnCharactersOnTargetPoints`
  (for (_array_element _array_index) (`self.SpawnTargets`)
    (bind _returnvalue (`|SpawnActorFromClass` "/Game/Assets/Carlos/Blueprints/PlayerCharacter.PlayerCharacter_C" (`self.GetTransform` _array_element) "AdjustIfPossibleButDontSpawnIfColliding" "OverrideRootScale" null null))
    (switch `int` _array_index
      (:`0`
        (set `/Game/Assets/Carlos/Blueprints/PlayerCharacter.CharacterSelection` (enumliteral `/Game/Characters/CharacterSelectionEnum` "NewEnumerator1") _returnvalue))
      (:`1`
        (set `/Game/Assets/Carlos/Blueprints/PlayerCharacter.CharacterSelection` (enumliteral `/Game/Characters/CharacterSelectionEnum` "NewEnumerator2") _returnvalue)))))

(fn `SpawnSpectatorCam`
  (returns (ReturnValue :type "/Game/Assets/Carlos/Blueprints/BP_SpectatorCamera Object Reference"))
  (bind _returnvalue (`GameplayStatics.GetPlayerCharacter` 0))
  (`/Engine/EditorBlueprintResources/StandardMacros.IsValid` _returnvalue
    (:`Is Valid`
      (bind _asplayer_character (cast `/Game/Assets/Carlos/Blueprints/PlayerCharacter` _returnvalue))
      (bind _returnvalue_2 (`|SpawnActorFromClass` "/Game/Assets/Carlos/Blueprints/BP_SpectatorCamera.BP_SpectatorCamera_C" (`KismetMathLibrary.MakeTransform` (`KismetMathLibrary.MakeVector` (.x (+ (.location (`SceneComponent.K2_GetComponentToWorld` (`/Game/Assets/Carlos/Blueprints/PlayerCharacter.Camera` _asplayer_character))) (* (`self.GetActorForwardVector` _asplayer_character) -250.0))) (.y (+ (.location (`SceneComponent.K2_GetComponentToWorld` (`/Game/Assets/Carlos/Blueprints/PlayerCharacter.Camera` _asplayer_character))) (* (`self.GetActorForwardVector` _asplayer_character) -250.0))) 1350.0)) "AdjustIfPossibleButAlwaysSpawn" "OverrideRootScale" null null))
      (return _returnvalue_2))))

(fn `UpdateHUD`
  (params (CharName :type Text) (MaxHp :type "Float (double-precision)") (CurrentHp :type "Float (double-precision)") (CharacterIcon :type "Texture2D Object Reference") (icon :type "Texture2D Object Reference") (icon2 :type "Texture2D Object Reference") (icon3 :type "Texture2D Object Reference"))
  (bind _asbp_hud_lovecraft (cast `/Game/UI/BP_HUD_Lovecraft` (`self.GetHUD`)))
  (`|ExecutionSequence`
    (:`then_0`
      (`/Game/UI/BP_HUD_Lovecraft.UpdateHP` _asbp_hud_lovecraft CharName MaxHp CurrentHp CharacterIcon))
    (:`then_1`
      (`/Game/UI/BP_HUD_Lovecraft.UpdateSkills` _asbp_hud_lovecraft icon icon2 icon3))))

(fn `UserConstructionScript`)