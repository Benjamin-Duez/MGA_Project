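; Player controller that shows a movement cost readout beside the mouse cursor.
; BeginPlay adds a Distance_WB widget to the viewport.
; Each tick, it runs ComputeCost from the Possessed actor to the point under the cursor, then writes the result into the widget and places it just above the mouse.
; The nodes meant to set Possessed from BP_TopDownCharacter are disconnected, so this graph never assigns it.
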(event `self.ReceiveBeginPlay`
  (bind _returnvalue (`|CreateWidget` "/Game/Blueprints/distance_WB.distance_WB_C"))
  (bind _output_get (set `self.distance` _returnvalue))
  (`UserWidget.AddToViewport` _output_get 0))

(event `self.ReceiveTick`
  (params (DeltaSeconds :type "Float (single-precision)"))
  (bind _returnvalue (`self.computeCost` self (`self.K2_GetActorLocation` (`self.possessed`)) (`.Location` (`GameplayStatics.BreakHitResult` (`self.GetHitResultUnderCursorByChannel` "TraceTypeQuery1")))))
  (`self.update_distance_WB` _returnvalue))

(fn `update_distance_WB`
  (params (Value :type "Float (single-precision)"))
  (bind (_locationx _locationy) (`self.GetMousePosition`))
  (bind _distance (`self.distance`))
  (`TextBlock.SetText` (`/Game/Blueprints/distance_WB.distance_txt` _distance) (`KismetTextLibrary.Conv_DoubleToText` Value "HalfToEven"))
  (`UserWidget.SetPositionInViewport` _distance (`KismetMathLibrary.MakeVector2D` (- _locationx 0.0) (- _locationy 25.0)) true))

(fn `UserConstructionScript`)